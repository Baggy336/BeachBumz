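; Tower1 is a tower that fires Tower1Bullets while enemies are within its detection radius.
; Overlap events add and remove EnemyCharacterBP actors in ListOfEnemies, and a DoOnce starts a looping Attack Enemy 1 timer on first entry.
; The timer spawns bullets at ShootingPoint's transform without passing a target.
; When the list empties, the timer is cleared and the DoOnce resets.
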(event OnComponentBeginOverlap(DetectionRadius)
  (params (OverlappedComponent :type Primitive%20Component%20Object%20Reference) (OtherActor :type Actor%20Object%20Reference) (OtherComp :type Primitive%20Component%20Object%20Reference) (OtherBodyIndex :type Integer) (bFromSweep :type Boolean) (SweepResult :type Hit%20Result%20Structure%20%28by%20ref%29))
  (bind _asenemy_character_bp (Utilities|Casting|CastToEnemyCharacterBP OtherActor))
  (Utilities|Array|Add (Variables|Default|GetList%20of%20Enemies) _asenemy_character_bp)
  (Utilities|FlowControl|DoOnce false
    (:Completed
      (Development|PrintString "Hello")
      (Utilities|Time|SetTimerbyFunctionName 0 "Attack Enemy 1" 0.8 true))))

(event OnComponentEndOverlap(DetectionRadius)
  (params (OverlappedComponent :type Primitive%20Component%20Object%20Reference) (OtherActor :type Actor%20Object%20Reference) (OtherComp :type Primitive%20Component%20Object%20Reference) (OtherBodyIndex :type Integer))
  (bind _list_of_enemies (Variables|Default|GetList%20of%20Enemies))
  (bind _asenemy_character_bp (Utilities|Casting|CastToEnemyCharacterBP OtherActor))
  (Utilities|Array|RemoveItem _list_of_enemies _asenemy_character_bp)
  (if (== (Utilities|Array|Length _list_of_enemies) 0)
    (Utilities|Time|ClearTimerbyFunctionName 0 "Attack Enemy 1")
    (Utilities|FlowControl|DoOnce false) ; enters at Reset
  ))

(fn ConstructionScript)

(fn AttackEnemy1
  (if (!= (Utilities|Array|Length (Variables|Default|GetList%20of%20Enemies)) 0)
    (Game|SpawnActorfromClass "/Game/Blueprints/Towers/Tower1Bullets.Tower1Bullets_C" (Transformation|GetWorldTransform (Variables|Default|GetShooting%20Point)) "Undefined" 0 0)))