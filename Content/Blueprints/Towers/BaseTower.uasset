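; Base tower actor for a tower defense game that automatically fires at enemies within its collider.
; Overlap begin and end events maintain a set of EnemyCharacterBP targets in range.
; From BeginPlay it loops on a short random delay, picking a random enemy from that set.
; Each shot spawns a Tower1Bullets actor at Point1, aimed ahead of the target using half a second of its velocity.
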(event OnComponentBeginOverlap(Collider)
  (params (OverlappedComponent :type Primitive%20Component%20Object%20Reference) (OtherActor :type Actor%20Object%20Reference) (OtherComp :type Primitive%20Component%20Object%20Reference) (OtherBodyIndex :type Integer) (bFromSweep :type Boolean) (SweepResult :type Hit%20Result%20Structure%20%28by%20ref%29))
  (bind _asenemy_character_bp (Utilities|Casting|CastToEnemyCharacterBP OtherActor))
  (Utilities|Set|Add (Variables|Default|Getenemies) _asenemy_character_bp))

(event OnComponentEndOverlap(Collider)
  (params (OverlappedComponent :type Primitive%20Component%20Object%20Reference) (OtherActor :type Actor%20Object%20Reference) (OtherComp :type Primitive%20Component%20Object%20Reference) (OtherBodyIndex :type Integer))
  (bind _asenemy_character_bp (Utilities|Casting|CastToEnemyCharacterBP OtherActor))
  (Utilities|Set|Remove (Variables|Default|Getenemies) _asenemy_character_bp))

(event Custom|Shoot%20at%20a%20random%20enemy
  (bind _enemies (Variables|Default|Getenemies))
  (if (> (Utilities|Set|Length _enemies) 0)
    (bind _result (Utilities|Set|ToArray _enemies))
    (CallFunction|ShootatEnemy (Utilities|Array|Get(acopy) _result (Math|Random|RandomIntegerinRange 0 (- (Utilities|Array|Length _result) 1))))))

(event Custom|Shoot%20at%20enemy
  (params (enemy :type Enemy%20Character%20BP%20Object%20Reference))
  (bind _point_1 (Variables|Default|GetPoint%201))
  (bind _returnvalue (Transformation|GetWorldLocation _point_1))
  (Game|SpawnActorfromClass "/Game/Blueprints/Towers/Tower1Bullets.Tower1Bullets_C" (Math|Transform|MakeTransform _returnvalue (Math|Rotator|FindLookatRotation _returnvalue (+ (Transformation|GetActorLocation enemy) (* (Transformation|GetVelocity enemy) 0.5))) "1,1,1") "Undefined" 0 0))

(event EventBeginPlay
  (Utilities|FlowControl|Delay (Math|Random|RandomFloatinRange 0.25 1.0) :!label _label)
  (CallFunction|ShootatARandomEnemy)
  (goto _label))

(fn ConstructionScript)