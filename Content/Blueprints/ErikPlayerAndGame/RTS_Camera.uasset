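; RTS camera pawn that serves as the player's view, moved by axis input and zoomed along a spring arm.
; On BeginPlay it becomes the player controller's view target and starts fully zoomed out.
; Forward and right axes feed movement input along the actor's own vectors, scaled by a speed multiplier.
; Zoom input adjusts a clamped target length, and the spring arm interpolates smoothly toward it.
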(event EventBeginPlay
  (Game|Player|SetViewTargetwithBlend (Game|GetPlayerController 0) self 0.0 "VTBlend_Linear" 0.0 false)
  (bind _output_get (Variables|/Script/Engine.SpringArmComponent|SetTargetArmLength (Variables|Default|GetSpringArm) (Variables|Default|GetMax_Zoom)))
  (Variables|Default|SetZoomTarget _output_get))

(event Input|AxisEvents|InputAxisMoveForward
  (params (AxisValue :type Float%20%28single-precision%29))
  (CallFunction|ForwardBackward AxisValue))

(event Input|AxisEvents|InputAxisMoveRight
  (params (AxisValue :type Float%20%28single-precision%29))
  (CallFunction|RightLeft AxisValue))

(event Input|AxisEvents|InputAxisCameraZoom
  (params (AxisValue :type Float%20%28single-precision%29))
  (CallFunction|Zoom AxisValue))

(fn ConstructionScript)

(fn ForwardBackward
  (params (Axis :type Float%20%28single-precision%29))
  (Pawn|Input|AddMovementInput (Transformation|GetActorForwardVector) (* (Variables|Default|GetSpeed_Multiplier) Axis) false))

(fn RightLeft
  (params (Axis :type Float%20%28single-precision%29))
  (Pawn|Input|AddMovementInput (Transformation|GetActorRightVector) (* (Variables|Default|GetSpeed_Multiplier) Axis) false))

(fn Zoom
  (params (Axis :type Float%20%28single-precision%29))
  (bind _springarm (Variables|Default|GetSpringArm))
  (bind _output_get (Variables|Default|SetZoomTarget (Math|Float|Clamp(Float) (+ (* Axis (Variables|Default|GetZoom_Multiplier)) (Variables|Default|GetZoomTarget)) (Variables|Default|GetMin_Zoom) (Variables|Default|GetMax_Zoom))))
  (Variables|/Script/Engine.SpringArmComponent|SetTargetArmLength _springarm (Math|Interpolation|FInterpTo (Variables|/Script/Engine.SpringArmComponent|GetTargetArmLength _springarm) _output_get (Utilities|Time|GetWorldDeltaSeconds) 15.0)))