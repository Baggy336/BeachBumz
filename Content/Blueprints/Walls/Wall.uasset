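; Destructible wall actor that tracks its health through a Wall_HealthBar widget component.
; BeginPlay seeds the widget with MaxHealth, and AnyDamage subtracts damage from Health, copies it to the widget and prints what remains.
; At zero or below, the wall destroys itself and sets CanSpawnAWall on the first Wall_BP_Area found in the level, allowing another wall to spawn.
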(event EventBeginPlay
  ;[1 1 1] Cast to health widget
  (bind _aswall_health_bar (Utilities|Casting|CastToWall_HealthBar (UserInterface|GetUserWidgetObject (Variables|Default|GetHealth%20Widget))))
  ;[1 1 1] Set max health
  (bind _output_get (Variables|Default|SetHealthWidgetRef _aswall_health_bar))
  (Variables|/Game/Blueprints/Walls/Wall_HealthBar.Wall_HealthBar_C|SetHealthRef _output_get (Variables|Stats|GetMax%20Health)))

(event Game|Damage|EventAnyDamage
  (params (Damage :type Float%20%28single-precision%29) (DamageType :type Damage%20Type%20Object%20Reference) (InstigatedBy :type Controller%20Object%20Reference) (DamageCauser :type Actor%20Object%20Reference))
  ;[1 1 1] When enemy is hit/how much damage they take
  (bind _output_get (Variables|Stats|SetHealth (- (Variables|Stats|GetHealth) Damage)))
  ;[1 1 1] Set the health in the widget
  (bind _output_get_2 (Variables|/Game/Blueprints/Walls/Wall_HealthBar.Wall_HealthBar_C|SetHealthRef (Variables|Default|GetHealthWidgetRef) _output_get))
  ;[1 1 1] Enemy Dies/ If enemy isn't dead print how much health it has
  (if (<= _output_get_2 0.0)
    (Actor|DestroyActor)
    ;[1 1 1] Can respawn wall
    (bind _outactors (Actor|GetAllActorsOfClass "/Game/Blueprints/Walls/Wall_BP_Area.Wall_BP_Area_C"))
    (bind _aswall_bp_area (Utilities|Casting|CastToWall_BP_Area (Utilities|Array|Get(acopy) _outactors)))
    (Variables|/Game/Blueprints/Walls/Wall_BP_Area.Wall_BP_Area_C|SetCanSpawnAWall _aswall_bp_area true)
    (else
      (Development|PrintString (Utilities|String|ToString(Float) _output_get_2)))))

(fn ConstructionScript)