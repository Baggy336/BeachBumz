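; Clickable wall build area for an RTS that opens a wall selection menu.
; Cursor hover, click and release events swap the mesh material as feedback, showing a disabled material on click when no wall can spawn.
; A valid click, if the game instance reports no widget enabled, clears existing WallSelection widgets, creates a new one linked to this area and sets that shared flag.
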(event OnBeginCursorOver(StaticMesh)
  (params (TouchedComponent :type Primitive%20Component%20Object%20Reference))
  (Rendering|Material|SetMaterial (Variables|Default|GetStaticMesh) 0 "/Game/Art/TowerBuilding/Materials/MouseOver.MouseOver"))

(event OnEndCursorOver(StaticMesh)
  (params (TouchedComponent :type Primitive%20Component%20Object%20Reference))
  (Rendering|Material|SetMaterial (Variables|Default|GetStaticMesh) 0 "/Game/Art/TowerBuilding/Materials/Default.Default"))

(event OnClicked(StaticMesh)
  (params (TouchedComponent :type Primitive%20Component%20Object%20Reference) (ButtonPressed :type Key%20Structure :default "None"))
  (bind _staticmesh (Variables|Default|GetStaticMesh))
  (if (Variables|Default|GetCanSpawnAWall)
    (Rendering|Material|SetMaterial _staticmesh 0 "/Game/Art/TowerBuilding/Materials/Clicked.Clicked")
    (bind _asrtsgame_instance (Utilities|Casting|CastToRTSGameInstance (Game|GetGameInstance)))
    (if (not (Variables|/Game/Blueprints/PlayerAndGame/RTSGameInstance.RTSGameInstance_C|GetisWidgetEnabled _asrtsgame_instance))
      (bind _foundwidgets (Widget|GetAllWidgetsOfClass "/Game/Blueprints/Walls/WallSelection.WallSelection_C" false))
      (for _array_element _foundwidgets
        (Widget|RemovefromParent _array_element))
      (bind _returnvalue (UserInterface|CreateWidget "/Game/Blueprints/Walls/WallSelection.WallSelection_C"))
      (UserInterface|Viewport|AddtoViewport _returnvalue 0)
      (Variables|/Game/Blueprints/Walls/WallSelection.WallSelection_C|SetWallArea _returnvalue self)
      (Variables|/Game/Blueprints/PlayerAndGame/RTSGameInstance.RTSGameInstance_C|SetisWidgetEnabled _asrtsgame_instance true))
    (else
      (Rendering|Material|SetMaterial _staticmesh 0 "/Game/Art/TowerBuilding/Materials/Disabled.Disabled"))))

(event OnReleased(StaticMesh)
  (params (TouchedComponent :type Primitive%20Component%20Object%20Reference) (ButtonReleased :type Key%20Structure :default "None"))
  (Rendering|Material|SetMaterial (Variables|Default|GetStaticMesh) 0 "/Game/Art/TowerBuilding/Materials/MouseOver.MouseOver"))

(event EventBeginPlay)

(event Collision|EventActorBeginOverlap
  (params (OtherActor :type Actor%20Object%20Reference)))

(event EventTick
  (params (DeltaSeconds :type Float%20%28single-precision%29)))

(fn ConstructionScript)