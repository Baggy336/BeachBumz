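; Base enemy character for an RTS that marches on the player's sandcastle, damaging it and destroying itself on arrival.
; A Tick-driven state machine moves between idle, walking, aggro and attack, using a forward line trace to target Walls or Allies and attack on a cooldown.
; Damage updates a health bar widget and destroys it at zero, with optional spawn and death FX.
; Bumping an enemy ahead launches it randomly sideways.
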(event OnComponentHit(CapsuleComponent)
  (params (HitComponent :type Primitive%20Component%20Object%20Reference) (OtherActor :type Actor%20Object%20Reference) (OtherComp :type Primitive%20Component%20Object%20Reference) (NormalImpulse :type Vector :default "0, 0, 0") (Hit :type Hit%20Result%20Structure%20%28by%20ref%29))
  (bind _asenemy_character_bp (Utilities|Casting|CastToEnemyCharacterBP OtherActor))
  (if (> (Math|Vector|DotProduct (Transformation|GetActorForwardVector) (Math|Vector|Normalize (- (Transformation|GetActorLocation _asenemy_character_bp) (Transformation|GetActorLocation)))) 0.0)
    (Character|LaunchCharacter (* (Math|Vector|SelectVector (Transformation|GetActorRightVector) (* (Transformation|GetActorRightVector) -1.0) (Math|Random|RandomBool)) 5e+02) false false)))

(event EventBeginPlay
  (bind _fx_at_spawn (Variables|Default|GetFX%20at%20spawn))
  (bind _asrtsgame_instance (Utilities|Casting|CastToRTSGameInstance (Game|GetGameInstance)))
  (Variables|Default|SetGameInstance _asrtsgame_instance)
  (Utilities|FlowControl|Sequence
    (:then_0
      ;[1 1 1] Set Speed
      (Variables|/Script/Engine.CharacterMovementComponent|SetMaxWalkSpeed (Variables|Character|GetCharacterMovement) (Math|Conversions|ToFloat(Integer) (Variables|Stats|GetSpeed)))
      ;[1 1 1] Set starting State
      (Variables|Default|SetCurrent%20State "NewEnumerator5"))
    (:then_1
      ;[1 1 1] Cast to health widget
      (bind _asai_health_bar (Utilities|Casting|CastToAI_HealthBar (UserInterface|GetUserWidgetObject (Variables|Default|GetHealth%20Widget))))
      ;[1 1 1] Set max health
      (bind _output_get (Variables|Default|SetHealthWidgetRef _asai_health_bar))
      (Variables|/Game/Blueprints/BaseAI/AI_HealthBar.AI_HealthBar_C|SetHealth _output_get (Variables|Stats|GetMaxHealth)))
    (:then_2
      (Variables|Default|SetAttack%20Target (Variables|/Game/Blueprints/PlayerAndGame/RTSGameInstance.RTSGameInstance_C|GetSandCastle (Variables|Default|GetGameInstance))))
    (:then_3
      (Utilities|IsValid _fx_at_spawn
        (:Is%20Valid
          (Niagara|SpawnSystematLocation _fx_at_spawn (Transformation|GetActorLocation)))))))

(event Game|Damage|EventAnyDamage
  (params (Damage :type Float%20%28single-precision%29) (DamageType :type Damage%20Type%20Object%20Reference) (InstigatedBy :type Controller%20Object%20Reference) (DamageCauser :type Actor%20Object%20Reference))
  ;[1 1 1] When enemy is hit/how much damage they take
  (bind _output_get (Variables|Stats|SetHealth (- (Variables|Stats|GetHealth) Damage)))
  ;[1 1 1] Set the health in the widget
  (bind _output_get_2 (Variables|/Game/Blueprints/BaseAI/AI_HealthBar.AI_HealthBar_C|SetHealth (Variables|Default|GetHealthWidgetRef) _output_get))
  ;[1 1 1] Enemy Dies/ If enemy isn't dead print how much health it has
  (if (<= _output_get_2 0.0)
    (Actor|DestroyActor)))

(event EventDestroyed
  (bind _fx_at_death (Variables|Default|GetFX%20at%20death))
  (Utilities|IsValid _fx_at_death
    (:Is%20Valid
      (Niagara|SpawnSystematLocation _fx_at_death (Transformation|GetActorLocation)))))

(event EventTick
  (params (DeltaSeconds :type Float%20%28single-precision%29))
  (bind _attack_target (Variables|Default|GetAttack%20Target))
  (switch Utilities|FlowControl|Switch|SwitchonBaseEnemyState (Variables|Default|GetCurrent%20State)
    (:NewEnumerator5
      ;[1 1 1] Delay for spawning so the AI can find the path
      (Utilities|FlowControl|Delay 0.2)
      (Variables|Default|SetCurrent%20State "NewEnumerator0"))
    (:NewEnumerator0
      ;[1 1 1] AI moves to Target
      (AI|AIMoveTo self "0, 0, 0" (Variables|/Game/Blueprints/PlayerAndGame/RTSGameInstance.RTSGameInstance_C|GetSandCastle (Variables|Default|GetGameInstance)) 1e+01 false
        (:then
          (CallFunction|RaycastLookforNearbyTargets)
          (Utilities|FlowControl|Delay 1.0)
          (CallFunction|SwitchtoState "NewEnumerator5"))
        (:OnSuccess
          (Variables|Default|SetCurrent%20State "NewEnumerator3"))))
    (:NewEnumerator1
      ;[1 1 1] Aggro towards enemy
      ;;[1 1 1] If target is destroyed go back to idle
      (Utilities|IsValid _attack_target
        (:Is%20Valid
          (AI|Navigation|SimpleMovetoActor (Pawn|GetController) _attack_target)
          (if (<= (Math|Vector|Distance(Vector) (Transformation|GetActorLocation) (Transformation|GetActorLocation (Variables|Default|GetAttack%20Target))) (Variables|Stats|GetDistanceNeededToAttack))
            (CallFunction|SwitchtoState "NewEnumerator6")))
        (:Is%20Not%20Valid
          (CallFunction|SwitchtoState "NewEnumerator5"))))
    (:NewEnumerator6
      ;[1 1 1] Attack the enemy and go back to aggro
      (bind _output_get (Variables|Stats|SetAttackCooldown (- (Variables|Stats|GetAttackCooldown) DeltaSeconds)))
      (if (<= _output_get 0.0)
        (CallFunction|SwitchtoState "NewEnumerator1")))
    (:NewEnumerator3
      ;[1 1 1] Destroys after spawning
      (Actor|DestroyActor)
      ;[1 1 1] Lower health of castle
      (bind _returnvalue (Actor|GetActorOfClass "/Game/Blueprints/PlayerAndGame/SandcastleBase.SandcastleBase_C"))
      (bind _assandcastle_base (Utilities|Casting|CastToSandcastleBase _returnvalue))
      (Variables|/Game/Blueprints/PlayerAndGame/SandcastleBase.SandcastleBase_C|SetcurrentHealth _assandcastle_base (- (Variables|/Game/Blueprints/PlayerAndGame/SandcastleBase.SandcastleBase_C|GetcurrentHealth _assandcastle_base) (Variables|Stats|GetDamageToCastle))))))

(fn ConstructionScript)

(fn SwitchtoState
  (params (New%20State :type BaseEnemyState%20Enum :default "NewEnumerator0"))
  (if (not (== New%20State (Variables|Default|GetCurrent%20State)))
    (bind _output_get (Variables|Default|SetCurrent%20State New%20State))
    (if (Utilities|Enum|Equal(Enum) _output_get "NewEnumerator6")
      (CallFunction|StartAttack))))

(fn RaycastLookforNearbyTargets
  (bind _returnvalue (Transformation|GetActorLocation))
  (bind (_outhit _returnvalue_2) (Collision|LineTraceByChannel _returnvalue (+ _returnvalue (* (Transformation|GetActorForwardVector) 275.0)) "TraceTypeQuery4" false 0 "ForOneFrame"))
  (if _returnvalue_2
    (bind _aswall (Utilities|Casting|CastToWall (.HitActor (Collision|BreakHitResult _outhit)))
      (:then
        (CallFunction|GoAggro _aswall))
      (:CastFailed
        ;[1 1 1] Cast to Friendly Unit
        (bind _asally (Utilities|Casting|CastToAlly (.HitActor (Collision|BreakHitResult _outhit))))
        (CallFunction|GoAggro _asally)))))

(fn GoAggro
  (params (Attack%20Target :type Actor%20Object%20Reference))
  (Variables|Default|SetAttack%20Target Attack%20Target)
  (CallFunction|SwitchtoState "NewEnumerator1"))

(fn StartAttack
  (Game|Damage|ApplyDamage (Variables|Default|GetAttack%20Target) (Variables|Stats|GetAttackDmg) 0 0)
  (Variables|Stats|SetAttackCooldown 5.0))