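; AI spawn point that runs enemy waves and opens the GameOverWin level when the wave count reaches 11.
; A timeline publishes a countdown to RTSGameInstance, and Tick calls the wave event while it reads zero.
; A looping timer spawns a random Clam or Golem nearby; the Bomb branch is unreachable with RandomInteger(2).
; HowManySpawn sets wave duration in seconds, not enemy count, and grows after each wave.
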(event Custom|Spawn%20Enemy
  (bind _returnvalue (Transformation|GetActorLocation))
  (bind _returnvalue_2 (Math|Random|RandomUnitVector))
  (bind _returnvalue_3 (* (.y _returnvalue_2) 5e+02))
  (bind _returnvalue_4 (* (.x _returnvalue_2) 5e+02))
  (bind _returnvalue_5 (+ (.y _returnvalue) _returnvalue_3))
  (bind _returnvalue_6 (+ (.x _returnvalue) _returnvalue_4))
  (bind _output_get (Variables|Default|SetWhichEnemy (Math|Random|RandomInteger 2)))
  (switch int _output_get
    (:Default
      (AI|SpawnAIFromClass "/Game/Blueprints/BaseAI/EnemyClasses/Clam.Clam_C" 0 (Math|Vector|MakeVector _returnvalue_6 _returnvalue_5 (.z _returnvalue)) "0, 0, 0" false 0 :!label _label))
    (:0
      (goto _label))
    (:1
      ;[1 1 1] Spawn on Location
      (AI|SpawnAIFromClass "/Game/Blueprints/BaseAI/EnemyClasses/Golem.Golem_C" 0 (Math|Vector|MakeVector _returnvalue_6 _returnvalue_5 (.z _returnvalue)) "0, 0, 0" false 0))
    (:2
      (AI|SpawnAIFromClass "/Game/Blueprints/BaseAI/EnemyClasses/Bomb.Bomb_C" 0 (Math|Vector|MakeVector _returnvalue_6 _returnvalue_5 (.z _returnvalue)) "0, 0, 0" false 0))))

(event Custom|SPAWWWN
  ;[1 1 1] Turn on Spawning
  (Utilities|Time|SetTimerbyEvent (delegate Custom|Spawn%20Enemy) (Variables|Default|GetSpawnTime) true)
  (Utilities|FlowControl|Delay (Math|Conversions|ToFloat(Integer) (Variables|Default|GetHowManySpawn)))
  ;[1 1 1] Turn off Spawning
  (Utilities|Time|SetTimerbyEvent (delegate Custom|Spawn%20Enemy) 0.01)
  (Variables|Default|SetWaveNumber (+ (Variables|Default|GetWaveNumber) 1))
  (Variables|Default|SetHowManySpawn (+ (Variables|Default|GetHowManySpawn) 1))
  (if (== (Variables|Default|GetWaveNumber) 11)
    (Game|OpenLevel(byName) "GameOverWin")))

(event EventBeginPlay
  (bind _asrtsgame_instance (Utilities|Casting|CastToRTSGameInstance (Game|GetGameInstance)))
  (Variables|/Game/Blueprints/PlayerAndGame/RTSGameInstance.RTSGameInstance_C|SetSpawnPoint _asrtsgame_instance self)
  (bind _spawntime (Timeline|SpawnTimer Play)
    (:Update
      (bind _asrtsgame_instance_2 (Utilities|Casting|CastToRTSGameInstance (Game|GetGameInstance)))
      (Variables|/Game/Blueprints/PlayerAndGame/RTSGameInstance.RTSGameInstance_C|SetSpawnTimer _asrtsgame_instance_2 (Math|Float|Truncate _spawntime)))))

(event EventTick
  (params (DeltaSeconds :type Float%20%28single-precision%29))
  (bind _asrtsgame_instance (Utilities|Casting|CastToRTSGameInstance (Game|GetGameInstance)))
  (if (== (Variables|/Game/Blueprints/PlayerAndGame/RTSGameInstance.RTSGameInstance_C|GetSpawnTimer _asrtsgame_instance) 0)
    (CallFunction|SPAWWWN)))

(fn ConstructionScript)