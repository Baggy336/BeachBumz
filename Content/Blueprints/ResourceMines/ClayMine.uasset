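; ClayMine is a clickable resource mine for an RTS that costs SandDollars to build and then produces Clay.
; A left click on its box opens the ClayMineBuilder widget, while BuildMine checks funds, deducts the cost and runs the Building timeline.
; Its state swaps a dynamic material texture between not built, in construction and built.
; Once built, Tick counts frames to periodically add Clay to PlayerDetails in the RTSGameInstance.
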(event OnClicked(Box)
  (params (TouchedComponent :type Primitive%20Component%20Object%20Reference) (ButtonPressed :type Key%20Structure :default "None"))
  (Development|PrintString "clicked")
  (if (== ButtonPressed "LeftMouseButton")
    (bind _returnvalue (UserInterface|CreateWidget "/Game/GUI/ResourceMineGUI/ClayMineBuilder.ClayMineBuilder_C"))
    (UserInterface|Viewport|AddtoViewport _returnvalue 0)))

(event Custom|Build%20Mine
  (bind _gameinstance (Variables|Default|GetGameInstance))
  (bind _playerdetails (Variables|/Game/Blueprints/PlayerAndGame/RTSGameInstance.RTSGameInstance_C|GetPlayerDetails _gameinstance))
  (if (Utilities|Enum|Equal(Enum) (Variables|Default|GetBuiltOrNot) "NewEnumerator1")
    (Development|PrintString (Utilities|String|ToString(Integer) (.sanddollars _playerdetails)))
    (if (> (.sanddollars _playerdetails) (Variables|Default|GetSandDollarsNeededToConstruct))
      (Development|PrintString "Constructing Mine")
      (CallFunction|ConstructingMine)
      (Timeline|Building Play
        (:Finished
          (Variables|Default|SetBuiltOrNot "NewEnumerator0")
          (CallFunction|ChangeTexture))))))

(event EventBeginPlay
  (Variables|Default|SetBuiltOrNot "NewEnumerator1")
  (CallFunction|ChangeTexture)
  (bind _asrtsgame_instance (Utilities|Casting|CastToRTSGameInstance (Game|GetGameInstance)))
  (Variables|Default|SetGameInstance _asrtsgame_instance))

(event EventTick
  (params (DeltaSeconds :type Float%20%28single-precision%29))
  (CallFunction|StoreClay))

(fn ConstructionScript
  (bind _returnvalue (Rendering|Material|CreateDynamicMaterialInstance (Variables|Default|GetCube) 0 "/Game/Art/Materials/StoneMineMAT.StoneMineMAT" "None" :!class /Script/Engine.PrimitiveComponent))
  (Variables|Default|SetStoneMineMAT _returnvalue)
  (CallFunction|ChangeTexture))

(fn ChangeTexture
  (Rendering|Material|SetTextureParameterValue (Variables|Default|GetStoneMineMAT) "Texture" (Utilities|Select :Index (Variables|Default|GetBuiltOrNot) :NewEnumerator0 "/Engine/EngineResources/AICON-Green_Low.AICON-Green" :NewEnumerator1 "/Engine/EngineResources/AICON-Red_Low.AICON-Red" :NewEnumerator2 "/Engine/EditorResources/Ai_Spawnpoint.Ai_Spawnpoint")))

(fn StoreClay
  (if (Utilities|Enum|Equal(Enum) (Variables|Default|GetBuiltOrNot) "NewEnumerator0")
    (Variables|Default|SetTimeBuilt (+ (Variables|Default|GetTimeBuilt) 1.0))
    (if (== (Variables|Default|GetTimeBuilt) (Variables|Default|GetGetStone))
      (bind _asrtsgame_instance (Utilities|Casting|CastToRTSGameInstance (Variables|Default|GetGameInstance)))
      (Variables|/Game/Blueprints/PlayerAndGame/RTSGameInstance.RTSGameInstance_C|SetPlayerDetails _asrtsgame_instance (Utilities|Struct|MakePlayerDetails (+ (.clay (Variables|/Game/Blueprints/PlayerAndGame/RTSGameInstance.RTSGameInstance_C|GetPlayerDetails _asrtsgame_instance)) 10) (.stone (Variables|/Game/Blueprints/PlayerAndGame/RTSGameInstance.RTSGameInstance_C|GetPlayerDetails _asrtsgame_instance)) (.sanddollars (Variables|/Game/Blueprints/PlayerAndGame/RTSGameInstance.RTSGameInstance_C|GetPlayerDetails _asrtsgame_instance))))
      (Development|PrintString (Utilities|String|ToString(Integer) (+ (.clay (Variables|/Game/Blueprints/PlayerAndGame/RTSGameInstance.RTSGameInstance_C|GetPlayerDetails _asrtsgame_instance)) 10)))
      (Variables|Default|SetTimeBuilt 0.0))))

(fn ConstructingMine
  (bind _gameinstance (Variables|Default|GetGameInstance))
  (Variables|Default|SetBuiltOrNot "NewEnumerator2")
  (CallFunction|ChangeTexture)
  (Variables|/Game/Blueprints/PlayerAndGame/RTSGameInstance.RTSGameInstance_C|SetPlayerDetails _gameinstance (Utilities|Struct|MakePlayerDetails (.clay (Variables|/Game/Blueprints/PlayerAndGame/RTSGameInstance.RTSGameInstance_C|GetPlayerDetails _gameinstance)) (.stone (Variables|/Game/Blueprints/PlayerAndGame/RTSGameInstance.RTSGameInstance_C|GetPlayerDetails _gameinstance)) (- (.sanddollars (Variables|/Game/Blueprints/PlayerAndGame/RTSGameInstance.RTSGameInstance_C|GetPlayerDetails _gameinstance)) (Variables|Default|GetSandDollarsNeededToConstruct)))))