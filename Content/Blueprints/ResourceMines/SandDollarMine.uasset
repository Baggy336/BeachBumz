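; Resource mine actor for sand dollars that shows its build state by swapping the texture on its cube mesh.
; The construction script creates a dynamic material instance, and ChangeTexture sets its texture parameter to a green icon for Built or red for NotBuilt.
; It starts NotBuilt, and any collider overlap begin or end toggles the state without filtering the other actor.
; The InConstruction state has no texture assigned.
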(event OnComponentBeginOverlap(Collider)
  (params (OverlappedComponent :type Primitive%20Component%20Object%20Reference) (OtherActor :type Actor%20Object%20Reference) (OtherComp :type Primitive%20Component%20Object%20Reference) (OtherBodyIndex :type Integer) (bFromSweep :type Boolean) (SweepResult :type Hit%20Result%20Structure%20%28by%20ref%29))
  (Variables|Default|SetBuiltOrNot "NewEnumerator0")
  (CallFunction|ChangeTexture))

(event OnComponentEndOverlap(Collider)
  (params (OverlappedComponent :type Primitive%20Component%20Object%20Reference) (OtherActor :type Actor%20Object%20Reference) (OtherComp :type Primitive%20Component%20Object%20Reference) (OtherBodyIndex :type Integer))
  (Variables|Default|SetBuiltOrNot "NewEnumerator1")
  (CallFunction|ChangeTexture))

(event EventBeginPlay
  (Variables|Default|SetBuiltOrNot "NewEnumerator1")
  (CallFunction|ChangeTexture))

(fn ConstructionScript
  (bind _returnvalue (Rendering|Material|CreateDynamicMaterialInstance (Variables|Default|GetCube) 0 "/Game/Art/Materials/SandDollarMineMAT.SandDollarMineMAT" "None" :!class /Script/Engine.PrimitiveComponent))
  (Variables|Default|SetSandDollarMineMAT _returnvalue)
  (CallFunction|ChangeTexture))

(fn ChangeTexture
  (Rendering|Material|SetTextureParameterValue (Variables|Default|GetSandDollarMineMAT) "Texture" (Utilities|Select :Index (Variables|Default|GetBuiltOrNot) :NewEnumerator0 "/Engine/EngineResources/AICON-Green.AICON-Green" :NewEnumerator1 "/Engine/EngineResources/AICON-Red.AICON-Red" :NewEnumerator2 0)))