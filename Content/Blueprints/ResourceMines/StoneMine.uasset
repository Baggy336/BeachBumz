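; Clickable RTS stone mine that is constructed by the player, then produces stone.
; A left click on an unbuilt mine checks Stone against the build cost, deducts SandDollars and advances the construction timer one step per call.
; Once built, a Tick counter periodically adds stone to RTSGameInstance's PlayerDetails, overwriting its other fields with constants.
; A dynamic material swaps textures to show not built, in construction or built.
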(event EventBeginPlay
  (Variables|Default|SetBuiltOrNot "NewEnumerator1")
  (CallFunction|ChangeTexture))

(event EventTick
  (params (DeltaSeconds :type Float%20%28single-precision%29))
  (CallFunction|StoreStone))

(event MouseInput|EventActorOnClicked
  (params (ButtonPressed :type Key%20Structure :default "None"))
  (if (== ButtonPressed "LeftMouseButton")
    (if (Utilities|Enum|Equal(Enum) (Variables|Default|GetBuiltOrNot) "NewEnumerator1")
      (if (> (.stone (Variables|/Game/Blueprints/PlayerAndGame/RTSGameInstance.RTSGameInstance_C|GetPlayerDetails (Variables|Default|GetGameInstance))) (Variables|Default|GetSandDollarsNeededToConstruct))
        (CallFunction|ConstructingMine)))))

(fn ConstructionScript
  (bind _returnvalue (Rendering|Material|CreateDynamicMaterialInstance (Variables|Default|GetCube) 0 "/Game/Art/Materials/StoneMineMAT.StoneMineMAT" "None" :!class /Script/Engine.PrimitiveComponent))
  (Variables|Default|SetStoneMineMAT _returnvalue)
  (CallFunction|ChangeTexture))

(fn ChangeTexture
  (Rendering|Material|SetTextureParameterValue (Variables|Default|GetStoneMineMAT) "Texture" (Utilities|Select :Index (Variables|Default|GetBuiltOrNot) :NewEnumerator0 "/Engine/EngineResources/AICON-Green_Low.AICON-Green" :NewEnumerator1 "/Engine/EngineResources/AICON-Red_Low.AICON-Red" :NewEnumerator2 "/Engine/EditorMaterials/Cascade/CASC_ModuleEnable.CASC_ModuleEnable")))

(fn StoreStone
  (if (Utilities|Enum|Equal(Enum) (Variables|Default|GetBuiltOrNot) "NewEnumerator0")
    (Variables|Default|SetTimeBuilt (+ (Variables|Default|GetTimeBuilt) 1.0))
    (if (== (Variables|Default|GetTimeBuilt) (Variables|Default|GetGetStone))
      (bind _asrtsgame_instance (Utilities|Casting|CastToRTSGameInstance (Variables|Default|GetGameInstance)))
      (Variables|/Game/Blueprints/PlayerAndGame/RTSGameInstance.RTSGameInstance_C|SetPlayerDetails _asrtsgame_instance (Utilities|Struct|MakePlayerDetails 0 (+ (.stone (Variables|/Game/Blueprints/PlayerAndGame/RTSGameInstance.RTSGameInstance_C|GetPlayerDetails _asrtsgame_instance)) 2) 600))
      (Development|PrintString (Utilities|String|ToString(Integer) (+ (.stone (Variables|/Game/Blueprints/PlayerAndGame/RTSGameInstance.RTSGameInstance_C|GetPlayerDetails _asrtsgame_instance)) 2)))
      (Variables|Default|SetTimeBuilt 0.0))))

(fn ConstructingMine
  (Variables|Default|SetBuiltOrNot "NewEnumerator2")
  (CallFunction|ChangeTexture)
  (bind _asrtsgame_instance (Utilities|Casting|CastToRTSGameInstance (Variables|Default|GetGameInstance)))
  (Variables|/Game/Blueprints/PlayerAndGame/RTSGameInstance.RTSGameInstance_C|SetPlayerDetails _asrtsgame_instance (Utilities|Struct|MakePlayerDetails 0 0 (- (.sanddollars (Variables|/Game/Blueprints/PlayerAndGame/RTSGameInstance.RTSGameInstance_C|GetPlayerDetails _asrtsgame_instance)) (Variables|Default|GetSandDollarsNeededToConstruct))))
  (if (< (Variables|Default|GetTimer) (Variables|Default|GetConstructionDone))
    (Variables|Default|SetTimer (+ (Variables|Default|GetTimer) 0.01))
    (else
      (Variables|Default|SetBuiltOrNot "NewEnumerator0")
      (CallFunction|ChangeTexture))))