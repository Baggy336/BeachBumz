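; Selectable RTS unit Blueprint with a Cylinder component that handles click selection.
; A left click on the Cylinder asks the RTS_Controller to remove the unit from the selection if UnitSelected is set, or add it otherwise.
; The IsSelected event applies UnitHover_MAT to the Cylinder and sets UnitSelected to true, ignoring its parameter, so nothing here clears the selected state.
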(event OnClicked(Cylinder)
  (params (TouchedComponent :type Primitive%20Component%20Object%20Reference) (ButtonPressed :type Key%20Structure))
  ;[1 1 1] If unit was left clicked
  (if (== ButtonPressed "LeftMouseButton")
    (bind _asrts_controller (Utilities|Casting|CastToRTS_Controller (Game|GetPlayerController 0)))
    (if (Variables|Default|GetunitSelected)
      (Default|RemoveUnitfromSelection _asrts_controller self)
      (else
        (Default|AddUnittoSelection _asrts_controller self)))))

(event Custom|IsSelected
  (params (isSelected :type Boolean))
  ;[1 1 1] When Unit is Selected
  (Rendering|Material|SetMaterial (Variables|Default|GetCylinder) 0 "/Game/Art/Materials/UnitHover_MAT.UnitHover_MAT")
  (Variables|Default|SetunitSelected true))

(event EventBeginPlay)

(fn ConstructionScript)