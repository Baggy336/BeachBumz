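; RTS player controller that handles mouse drag-to-select and tracks which units are selected.
; On BeginPlay it locks the mouse in Game and UI input mode with the cursor visible during capture.
; Left mouse press and release send start and stop selection messages to the HUD.
; Add and remove functions maintain a unique array of selected units and set each unit's selected state.
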(event EventBeginPlay
  (Input|SetInputModeGameandUI self 0 "LockAlways" false))

(event Input|MouseEvents|LeftMouseButton
  (params (Key :type Key%20Structure))
  (bind _returnvalue (HUD|GetHUD))
  ;[1 1 1] Start/Stop Drag to Select
  (:Pressed
    (Class|SelectionInterface|StartSelection(Message) _returnvalue))
  (:Released
    (Class|SelectionInterface|StopSelection(Message) _returnvalue)))

(fn ConstructionScript)

(fn AddUnittoSelection
  (params (Selectable_Unit :type Selectable%20Unit%20Object%20Reference))
  ;[1 1 1] Add Selected Unit to Array
  (Utilities|Array|AddUnique (Variables|Default|GetSelected%20Unit) Selectable_Unit)
  (Default|IsSelected Selectable_Unit true))

(fn RemoveUnitfromSelection
  (params (Selectable_Unit :type Selectable%20Unit%20Object%20Reference))
  ;[1 1 1] Remove Deselected Unit from Array
  (Utilities|Array|RemoveItem (Variables|Default|GetSelected%20Unit) Selectable_Unit)
  (Default|IsSelected Selectable_Unit false))