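; ThePlayer is the player-side Blueprint that issues move orders to selected Ally units in what appears to be RTS-style control.
; On a right-click press it loops over every Ally actor in the level and calls Move on those flagged IsSelected.
; Two unconnected leftover chains would instead call StopMovingTo or MovingTo on the first MyAIController found, but they never run.
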(event Input|ActionEvents|InputActionRightClick
  (params (Key :type Key%20Structure))
  (:Pressed
    (bind _outactors (Actor|GetAllActorsOfClass "/Game/Blueprints/PlayerAndGame/Ally.Ally_C"))
    (for _array_element _outactors
      (if (Variables|/Game/Blueprints/PlayerAndGame/Ally.Ally_C|GetIs%20Selected? _array_element)
        (Default|Move _array_element)))))

(fn ConstructionScript)