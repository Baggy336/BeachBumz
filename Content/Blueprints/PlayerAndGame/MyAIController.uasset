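; AI controller that moves its pawn toward the point under the first player's mouse cursor, for hold-to-move control.
; MovingTo and StopMovingTo open and close a gate on Tick, which traces the Visibility channel under the cursor each frame while open.
; MoveToLocation issues a simple move to the hit point unless it lies too close to the pawn.
; An IsDead check on the pawn is present but never runs.
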(event Custom|Moving%20To
  (Utilities|FlowControl|Gate true) ; enters at Open
)

(event Custom|Stop%20Moving%20To
  (Utilities|FlowControl|Gate true) ; enters at Close
)

(event EventTick
  (params (DeltaSeconds :type Float%20%28single-precision%29))
  (Utilities|FlowControl|Gate true ; While key is pressed...
    (:Exit
      (CallFunction|MovetoLocation (.HitResult (Game|Player|GetHitResultUnderCursorbyChannel (Game|GetPlayerController 0) "TraceTypeQuery1" true))) ; ...and move there
    )))

(event Input|ActionEvents|InputActionRightClick
  (params (Key :type Key%20Structure)))

(fn ConstructionScript)

(fn MovetoLocation
  (params (Hit :type Hit%20Result%20Structure))
  (bind _location (Collision|BreakHitResult Hit))
  (if (>= (Math|Vector|VectorLength (- (Transformation|GetActorLocation (Pawn|GetControlledPawn)) _location)) 1.2e+02) ; Don't move if player clicks too close to pawn
    (AI|Navigation|SimpleMovetoLocation self _location)))