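; Player's sandcastle base for the RTS, which registers itself with RTSGameInstance and opens the lose level when its health runs out.
; Tick accumulates time to add Sand Dollars to the game instance, while overlapping enemies subtract their attack damage from health.
; LevelUp raises health and sets the income interval at higher levels.
; Selection events open the base overlay widget, and SpawnUnit runs a progress timeline before spawning an Ally and deducting Clay.
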(event OnComponentBeginOverlap(BoxCollision)
  (params (OverlappedComponent :type Primitive%20Component%20Object%20Reference) (OtherActor :type Actor%20Object%20Reference) (OtherComp :type Primitive%20Component%20Object%20Reference) (OtherBodyIndex :type Integer) (bFromSweep :type Boolean) (SweepResult :type Hit%20Result%20Structure%20%28by%20ref%29))
  (bind _asenemy_character_bp (Utilities|Casting|CastToEnemyCharacterBP OtherActor))
  (Variables|Default|SetcurrentHealth (- (Variables|Default|GetcurrentHealth) (Math|Float|Truncate (Variables|/Game/Blueprints/BaseAI/EnemyCharacterBP.EnemyCharacterBP_C|GetAttackDmg _asenemy_character_bp)))))

(event Custom|LevelUp
  (Variables|Default|Setlevel (+ (Variables|Default|Getlevel) 1))
  (Variables|Default|SetmaxHealth (+ (Variables|Default|GetmaxHealth) 500))
  (Variables|Default|SetcurrentHealth (+ (Variables|Default|GetcurrentHealth) 500))
  (if (> (Variables|Default|GetcurrentHealth) (Variables|Default|GetmaxHealth))
    (Variables|Default|SetcurrentHealth (Variables|Default|GetmaxHealth)))
  (if (>= (Variables|Default|Getlevel) 3)
    (Variables|Default|SetsandDollarGenRate 2.5)))

(event Custom|Spawn%20Unit
  (bind _spawnpoint (Variables|Default|GetSpawnpoint))
  (bind _gameinstance (Variables|Default|GetgameInstance))
  (bind _returnvalue (Transformation|GetWorldLocation _spawnpoint))
  (if (> (.clay (Variables|/Game/Blueprints/PlayerAndGame/RTSGameInstance.RTSGameInstance_C|GetPlayerDetails (Variables|Default|GetgameInstance))) 50)
    (bind _percent (Timeline|Spawntimer PlayFromStart)
      (:Update
        (Variables|Default|SetSpawntime _percent))
      (:Finished
        (Game|SpawnActorfromClass "/Game/Blueprints/PlayerAndGame/Ally.Ally_C" (Math|Transform|MakeTransform (Math|Vector|MakeVector (.x _returnvalue) (.y _returnvalue) 0.0) "0, 0, 0" "1,1,1") "Undefined" 0 0)
        (Variables|/Game/Blueprints/PlayerAndGame/RTSGameInstance.RTSGameInstance_C|SetPlayerDetails _gameinstance (Utilities|Struct|MakePlayerDetails (- (.clay (Variables|/Game/Blueprints/PlayerAndGame/RTSGameInstance.RTSGameInstance_C|GetPlayerDetails _gameinstance)) 50) (.stone (Variables|/Game/Blueprints/PlayerAndGame/RTSGameInstance.RTSGameInstance_C|GetPlayerDetails _gameinstance)) (.sanddollars (Variables|/Game/Blueprints/PlayerAndGame/RTSGameInstance.RTSGameInstance_C|GetPlayerDetails _gameinstance))))
        (Variables|Default|SetSpawntime 0.0)))))

(event EventBeginPlay
  (bind _asrtsgame_instance (Utilities|Casting|CastToRTSGameInstance (Game|GetGameInstance)))
  (bind _output_get (Variables|Default|SetgameInstance _asrtsgame_instance))
  (Variables|/Game/Blueprints/PlayerAndGame/RTSGameInstance.RTSGameInstance_C|SetSandCastle _output_get self))

(event Collision|EventActorBeginOverlap
  (params (OtherActor :type Actor%20Object%20Reference)))

(event EventTick
  (params (DeltaSeconds :type Float%20%28single-precision%29))
  (bind _gameinstance (Variables|Default|GetgameInstance))
  (Utilities|FlowControl|Sequence
    (:then_0
      (bind _output_get (Variables|Default|SetdeltaSecondsAdded (+ DeltaSeconds (Variables|Default|GetdeltaSecondsAdded))))
      (if (>= _output_get (Variables|Default|GetsandDollarGenRate))
        (Variables|Default|SetdeltaSecondsAdded (- (Variables|Default|GetdeltaSecondsAdded) (Variables|Default|GetsandDollarGenRate)))
        (Variables|/Game/Blueprints/PlayerAndGame/RTSGameInstance.RTSGameInstance_C|SetPlayerDetails _gameinstance (Utilities|Struct|MakePlayerDetails (.Clay (Utilities|Struct|BreakPlayerDetails (Variables|/Game/Blueprints/PlayerAndGame/RTSGameInstance.RTSGameInstance_C|GetPlayerDetails _gameinstance))) (.Stone (Utilities|Struct|BreakPlayerDetails (Variables|/Game/Blueprints/PlayerAndGame/RTSGameInstance.RTSGameInstance_C|GetPlayerDetails _gameinstance))) (+ (.SandDollars (Utilities|Struct|BreakPlayerDetails (Variables|/Game/Blueprints/PlayerAndGame/RTSGameInstance.RTSGameInstance_C|GetPlayerDetails _gameinstance))) 1)))
        (Development|PrintString (Utilities|String|ToString(Integer) (+ (.SandDollars (Utilities|Struct|BreakPlayerDetails (Variables|/Game/Blueprints/PlayerAndGame/RTSGameInstance.RTSGameInstance_C|GetPlayerDetails _gameinstance))) 1)))))
    (:then_1
      (if (<= (Variables|Default|GetcurrentHealth) 0)
        (Development|PrintString "Base is Dead")
        (Game|OpenLevel(byObjectReference) "/Game/Map/UIMaps/GameOverLose.GameOverLose")))))

(event EventBuildingIsSelected
  (params (Is%20Selected :type Boolean))
  (bind _gameinstance (Variables|Default|GetgameInstance))
  (if (not (Variables|/Game/Blueprints/PlayerAndGame/RTSGameInstance.RTSGameInstance_C|GetisWidgetEnabled _gameinstance))
    (if (not Is%20Selected)
      (bind _output_get (Variables|Default|SetisSelected false))
      (Rendering|Material|SetMaterial (Variables|Default|GetCube) 0 (select _output_get "/Game/Art/Materials/UnitHover_MAT.UnitHover_MAT" "/Engine/BasicShapes/BasicShapeMaterial.BasicShapeMaterial"))
      (if true
        (bind _returnvalue (UserInterface|CreateWidget "/Game/GUI/SandcastleBaseOverlay.SandcastleBaseOverlay_C"))
        (UserInterface|Viewport|AddtoViewport _returnvalue 0)
        (Variables|/Game/Blueprints/PlayerAndGame/RTSGameInstance.RTSGameInstance_C|SetisWidgetEnabled _gameinstance true)))))

(fn ConstructionScript
  (|CallParentFunction))