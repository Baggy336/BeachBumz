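; RTS player controller that sets Game-and-UI input with a locked cursor, adds the overlay UI and tracks the player's selection.
; Left mouse tells the HUD to start and stop drag selection, while Ctrl and Shift set held-state flags.
; Helper functions maintain selected unit and building arrays and their highlight states, with unit adding toggling the state.
; Ctrl+1 adds only the first selected unit to control group 1.
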(event EventBeginPlay
  (Input|SetInputModeGameandUI self 0 "LockAlways" false)
  (bind _asrtsgame_instance (Utilities|Casting|CastToRTSGameInstance (Game|GetGameInstance)))
  (Variables|Default|SetGameInstance _asrtsgame_instance)
  (bind _returnvalue (UserInterface|CreateWidget "/Game/GUI/OverlayUI.OverlayUI_C"))
  (bind _output_get (Variables|Default|SetOverlayUI _returnvalue))
  (UserInterface|Viewport|AddtoViewport _output_get 0))

(event Input|MouseEvents|LeftMouseButton
  (params (Key :type Key%20Structure :default "None"))
  (bind _returnvalue (HUD|GetHUD))
  ;[1 1 1] Start/Stop Drag to Select
  (:Pressed
    (Class|SelectionInterface|StartSelection(Message) _returnvalue))
  (:Released
    (Class|SelectionInterface|StopSelection(Message) _returnvalue)))

(event Input|KeyboardEvents|LeftCtrl
  (params (Key :type Key%20Structure :default "None"))
  ;[1 1 1] Detect When CTRL or SHIFT are being Held
  (:Pressed
    (Variables|Default|SetisHoldingControl true))
  (:Released
    (Variables|Default|SetisHoldingControl false)))

(event Input|KeyboardEvents|LeftShift
  (params (Key :type Key%20Structure :default "None"))
  ;[1 1 1] Detect When CTRL or SHIFT are being Held
  (:Pressed
    (Variables|Default|SetisHoldingShift true))
  (:Released
    (Variables|Default|SetisHoldingShift false)))

(event Input|KeyboardEvents|1
  (params (Key :type Key%20Structure :default "None"))
  (:Pressed
    (if (Variables|Default|GetisHoldingControl)
      (CallFunction|AddtoControlGroup1 (Utilities|Array|Get(acopy) (Variables|Default|GetSelected%20Unit))))))

(fn ConstructionScript)

(fn AddUnittoSelection
  (params (Selectable_Unit :type Ally%20Object%20Reference))
  ;[1 1 1] Add Selected Unit to Array
  (Utilities|Array|AddUnique (Variables|Default|GetSelected%20Unit) Selectable_Unit)
  (Default|IsSelected Selectable_Unit (not (Variables|/Game/Blueprints/PlayerAndGame/Ally.Ally_C|GetIs%20Selected? Selectable_Unit))))

(fn RemoveUnitfromSelection
  (params (Selectable_Unit :type Ally%20Object%20Reference))
  ;[1 1 1] Remove Deselected Unit from Array
  (Utilities|Array|RemoveItem (Variables|Default|GetSelected%20Unit) Selectable_Unit)
  (Default|IsSelected Selectable_Unit false))

(fn ClearSelection
  ;[1 1 1] Deselect every unit in array
  (for _array_element (Variables|Default|GetSelected%20Unit)
    (Default|IsSelected _array_element false))
  (Utilities|Array|Clear (Variables|Default|GetSelected%20Unit)) ; Remove all units from array
  ;[1 1 1] Deselect every building in array
  (for _array_element_2 (Variables|Default|GetSelected%20Building)
    (Default|BuildingIsSelected _array_element_2 false))
  (Utilities|Array|Clear (Variables|Default|GetSelected%20Building)) ; Remove all buildings from array
)

(fn AddBuildingtoSelection
  (params (Selectable_Building :type Selectable%20Building%20Object%20Reference))
  ;[1 1 1] Add Selected Building to Array
  (Utilities|Array|AddUnique (Variables|Default|GetSelected%20Building) Selectable_Building)
  (Default|BuildingIsSelected Selectable_Building true))

(fn RemoveBuildingfromSelection
  (params (Selectable_Building :type Selectable%20Building%20Object%20Reference))
  ;[1 1 1] Remove Deselected Building from Array
  (Utilities|Array|RemoveItem (Variables|Default|GetSelected%20Building) Selectable_Building)
  (Default|BuildingIsSelected Selectable_Building false))

(fn AddtoControlGroup1
  (params (NewItem :type Object%20Object%20Reference%20%28by%20ref%29))
  (Utilities|Array|AddUnique (Variables|Default|GetControl%20Group%201) NewItem))