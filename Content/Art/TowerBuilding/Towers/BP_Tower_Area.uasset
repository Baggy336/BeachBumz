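; BP_Tower_Area is a clickable build spot for placing towers.
; Cursor and click events on its static mesh swap materials for hover, default, clicked and disabled feedback.
; When a tower can spawn, a click removes any open TowerSelection widgets, then creates a new one and passes it a reference to this area.
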(event OnBeginCursorOver(StaticMesh)
  (params (TouchedComponent :type Primitive%20Component%20Object%20Reference))
  (Rendering|Material|SetMaterial (Variables|Default|GetStaticMesh) 0 "/Game/Art/TowerBuilding/Materials/MouseOver.MouseOver"))

(event OnEndCursorOver(StaticMesh)
  (params (TouchedComponent :type Primitive%20Component%20Object%20Reference))
  (Rendering|Material|SetMaterial (Variables|Default|GetStaticMesh) 0 "/Game/Art/TowerBuilding/Materials/Default.Default"))

(event OnClicked(StaticMesh)
  (params (TouchedComponent :type Primitive%20Component%20Object%20Reference) (ButtonPressed :type Key%20Structure))
  (bind _staticmesh (Variables|Default|GetStaticMesh))
  (if (Variables|Default|GetCanSpawnATower)
    (Rendering|Material|SetMaterial _staticmesh 0 "/Game/Art/TowerBuilding/Materials/Clicked.Clicked")
    (bind _foundwidgets (Widget|GetAllWidgetsOfClass "/Game/Art/TowerBuilding/Towers/TowerSelection.TowerSelection_C" false))
    (for _array_element _foundwidgets
      (Widget|RemovefromParent _array_element))
    (bind _returnvalue (UserInterface|CreateWidget "/Game/Art/TowerBuilding/Towers/TowerSelection.TowerSelection_C"))
    (UserInterface|Viewport|AddtoViewport _returnvalue 0)
    (Variables|/Game/Art/TowerBuilding/Towers/TowerSelection.TowerSelection_C|SetTowerArea _returnvalue self)
    (else
      (Rendering|Material|SetMaterial _staticmesh 0 "/Game/Art/TowerBuilding/Materials/Disabled.Disabled"))))

(event OnReleased(StaticMesh)
  (params (TouchedComponent :type Primitive%20Component%20Object%20Reference) (ButtonReleased :type Key%20Structure))
  (Rendering|Material|SetMaterial (Variables|Default|GetStaticMesh) 0 "/Game/Art/TowerBuilding/Materials/MouseOver.MouseOver"))

(event EventBeginPlay)

(event Collision|EventActorBeginOverlap
  (params (OtherActor :type Actor%20Object%20Reference)))

(event EventTick
  (params (DeltaSeconds :type Float%20%28single-precision%29)))

(fn ConstructionScript)